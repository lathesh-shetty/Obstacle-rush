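; Game mode that tracks collectibles, opens the gate when none remain, and persists collected state to a save game.
; Collectibles register to raise a counter; each collection lowers it, records the object's ID, updates the UI, checks for completion and saves asynchronously.
; On BeginPlay it loads or creates the save, then replays state by calling a savable-state interface on actors whose IDs are stored; EndPlay also saves.
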(event `SaveGame`
  ;[1 1 1] Save our Save Game Object to storage
  (`AsyncActionHandleSaveGame.AsyncSaveGameToSlot` (`self.SaveGameRef`) (`.SlotName` (defaults `/Game/BlueprintSaveLoad/Classes/FINISHED/SG_Collectible_FINISHED` "/Game/BlueprintSaveLoad/Classes/FINISHED/SG_Collectible_FINISHED.SG_Collectible_FINISHED_C"))))

(event `LoadSaveGame`
  ;[1 1 1] Load our Save Game from storage into a reference then call the change state event on all items that can accept it
  (bind _returnvalue (`GameplayStatics.DoesSaveGameExist` (`.SlotName` (defaults `/Game/BlueprintSaveLoad/Classes/FINISHED/SG_Collectible_FINISHED` "/Game/BlueprintSaveLoad/Classes/FINISHED/SG_Collectible_FINISHED.SG_Collectible_FINISHED_C"))))
  (if _returnvalue
    (bind _returnvalue_2 (`GameplayStatics.LoadGameFromSlot` (`.SlotName` (defaults `/Game/BlueprintSaveLoad/Classes/FINISHED/SG_Collectible_FINISHED` "/Game/BlueprintSaveLoad/Classes/FINISHED/SG_Collectible_FINISHED.SG_Collectible_FINISHED_C"))))
    (bind _assg_collectible_finished (cast `/Game/BlueprintSaveLoad/Classes/FINISHED/SG_Collectible_FINISHED` _returnvalue_2))
    (bind _output_get (set `self.SaveGameRef` _assg_collectible_finished))
    (`self.ChangeStateOnSavedObjects` (`/Game/BlueprintSaveLoad/Classes/FINISHED/SG_Collectible_FINISHED.ObjectsWithChangedState` _output_get))
    (else
      (bind _returnvalue_3 (`GameplayStatics.CreateSaveGameObject` "/Game/BlueprintSaveLoad/Classes/FINISHED/SG_Collectible_FINISHED.SG_Collectible_FINISHED_C"))
      (set `self.SaveGameRef` _returnvalue_3))))

(event `RegisterCollectible`
  ;[1 1 1] A Collectible wants to register with us
  (bind _result (`/Engine/EditorBlueprintResources/StandardMacros.IncrementInt` (`self.NumItemsToCollect`))
    (:`  `
      (`KismetSystemLibrary.PrintString` (`KismetStringLibrary.Conv_IntToString` _result)))))

(event `CollectibleCollected`
  (params (ID :type String))
  ;[1 1 1] Collectible was Collected, remove it from our number of items to collect then register it in our Save Game object, then see if we have collected them all and open the door if we have, then finally save the game since we did something
  (bind _result (`/Engine/EditorBlueprintResources/StandardMacros.DecrementInt` (`self.NumItemsToCollect`))
    (:`  `
      (`KismetSystemLibrary.PrintString` (`KismetStringLibrary.Conv_IntToString` _result))
      (`KismetArrayLibrary.Array_AddUnique` (`/Game/BlueprintSaveLoad/Classes/FINISHED/SG_Collectible_FINISHED.ObjectsWithChangedState` (`self.SaveGameRef`)) ID)
      (`self.UpdateCollectibleUI`)
      (bind _alldestroyed (`self.CheckForAllCollectiblesDestroyed`))
      (if _alldestroyed
        (`self.OpenMasterDoor`))
      (`self.SaveGame`))))

(event `self.ReceiveBeginPlay`
  ;[1 1 1] Begin Play - Load our Save Game
  (`self.LoadSaveGame`)
  (`KismetSystemLibrary.Delay` 0.2)
  (`self.UpdateCollectibleUI`))

(event `self.ReceiveEndPlay`
  (params (EndPlayReason :type "EEndPlayReason Enum" :default "Destroyed"))
  ;[1 1 1] End Play - Save our game as we end the game
  (`self.SaveGame`))

(fn `ChangeStateOnSavedObjects`
  (params (InputObjects :type "Array of String"))
  (bind _outactors (`GameplayStatics.GetAllActorsWithInterface` "/Game/BlueprintSaveLoad/Classes/FINISHED/BPI_SavableState_FINISHED.BPI_SavableState_FINISHED_C"))
  (for _array_element _outactors
    (bind _id (message `/Game/BlueprintSaveLoad/Classes/FINISHED/BPI_SavableState_FINISHED.GetID` _array_element))
    (if (`KismetArrayLibrary.Array_Contains` InputObjects _id)
      (message `/Game/BlueprintSaveLoad/Classes/FINISHED/BPI_SavableState_FINISHED.ChangeState` _array_element))))

(fn `CheckForAllCollectiblesDestroyed`
  (returns (AllDestroyed :type Boolean))
  (return (<= (`self.NumItemsToCollect`) 0)))

(fn `OpenMasterDoor`
  ;[1 1 1] Get our door, open it
  (bind _returnvalue (`GameplayStatics.GetActorOfClass` "/Game/BlueprintSaveLoad/Blueprints/FINISHED/BP_Gate_FINISHED.BP_Gate_FINISHED_C"))
  (`/Game/BlueprintSaveLoad/Blueprints/FINISHED/BP_Gate_FINISHED.OpenDoor` _returnvalue))

(fn `UpdateCollectibleUI`
  (`/Game/BlueprintSaveLoad/UMG/FINISHED/UMG_PlayerUI_FINISHED.SetCollectibleDisplay` (`self.PlayerUIRef`) (`self.NumItemsToCollect`)))

(fn `UserConstructionScript`)